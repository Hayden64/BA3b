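; BP_BaseBuilding is a base building Blueprint that charges the player money and reports its economy effects.
; On BeginPlay it caches MainGameInstance and BP_BaseController.
; Interact deducts Cost from DisplayedMoney when affordable, then passes money, population and happiness multipliers to the game instance.
; Despite its name, Remove only sets the controller's HasMoney flag; crew count and happiness functions exist but are not called here.
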(event EventBeginPlay
  (bind _asmain_game_instance (Utilities|Casting|CastToMainGameInstance (Game|GetGameInstance)))
  (Variables|Default|SetAs%20Main%20Game%20Instance _asmain_game_instance)
  (bind _asbp_base_controller (Utilities|Casting|CastToBP_BaseController (Game|GetPlayerController 0)))
  (Variables|Default|SetAs%20BP%20Base%20Controller _asbp_base_controller))

(event EventRemove
  (bind _as_bp_base_controller (Variables|Default|GetAs%20BP%20Base%20Controller))
  ;[1 1 1] Removes money
  (if (> (Variables|Recourse|Getcost) (Variables|/Game/FMP/Camera/MainGameInstance.MainGameInstance_C|GetDisplayed%20Money (Variables|Default|GetAs%20Main%20Game%20Instance)))
    (Variables|/Game/FMP/Camera/BP_BaseController.BP_BaseController_C|SetHas%20Money _as_bp_base_controller false)
    (else
      (Variables|/Game/FMP/Camera/BP_BaseController.BP_BaseController_C|SetHas%20Money _as_bp_base_controller true))))

(event EventInteract
  (if (not (> (Variables|Recourse|Getcost) (Variables|/Game/FMP/Camera/MainGameInstance.MainGameInstance_C|GetDisplayed%20Money (Variables|Default|GetAs%20Main%20Game%20Instance))))
    (CallFunction|ChangeMoney)
    (Class|BPInterface|PassBuildingInfo(Message) (Game|GetGameInstance) (Variables|Multiplyers|GetMoney%20Multiplyer) (Variables|Multiplyers|GetPopulation%20Multiplyer) (Variables|Multiplyers|GetHappines%20Multiplyer))))

(fn ConstructionScript)

(fn ChangeMoney
  (bind _as_main_game_instance (Variables|Default|GetAs%20Main%20Game%20Instance))
  (Variables|/Game/FMP/Camera/MainGameInstance.MainGameInstance_C|SetDisplayed%20Money _as_main_game_instance (- (Variables|/Game/FMP/Camera/MainGameInstance.MainGameInstance_C|GetDisplayed%20Money _as_main_game_instance) (Variables|Recourse|Getcost))))

(fn ChangeCrewNum
  (bind _as_main_game_instance (Variables|Default|GetAs%20Main%20Game%20Instance))
  (Variables|/Game/FMP/Camera/MainGameInstance.MainGameInstance_C|SetDisplayed%20Population _as_main_game_instance (+ (Variables|/Game/FMP/Camera/MainGameInstance.MainGameInstance_C|GetDisplayed%20Population _as_main_game_instance) (Variables|Recourse|GetCrew%20Num))))

(fn ChangeHappenis
  (bind _as_main_game_instance (Variables|Default|GetAs%20Main%20Game%20Instance))
  (Variables|/Game/FMP/Camera/MainGameInstance.MainGameInstance_C|SetDisplayed%20Crew%20Happiness _as_main_game_instance (+ (Variables|/Game/FMP/Camera/MainGameInstance.MainGameInstance_C|GetDisplayed%20Crew%20Happiness _as_main_game_instance) (Variables|Recourse|GetCrew%20Happiness))))