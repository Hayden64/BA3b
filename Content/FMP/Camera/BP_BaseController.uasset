(event Custom|Can%20Follow%20Mouse
  ;[0.6118 1 0.5529] Follow and unfollow mouse pos
  (Variables|Default|SetFollowMouse true))

(event Custom|Stops%20Following%20mouse
  ;[0.6118 1 0.5529] Follow and unfollow mouse pos
  (Variables|Default|SetFollowMouse false))

(event Input|EnhancedActionEvents|EnhancedInputActionIA_CameraMove
  (params (ActionValue :type Vector%202D%20Structure) (ElapsedSeconds :type Float%20%28double-precision%29) (TriggeredSeconds :type Float%20%28double-precision%29) (InputAction :type Input%20Action%20Object%20Reference :default "/Game/FMP/Camera/Input/EnhancedInput/IA_CameraMove.IA_CameraMove"))
  ;[1 0.6314 0.8938] Movement
  (Camera|Moving (.x ActionValue) (.y ActionValue)))

(event Input|EnhancedActionEvents|EnhancedInputActionIA_Zoom
  (params (ActionValue :type Float%20%28double-precision%29) (ElapsedSeconds :type Float%20%28double-precision%29) (TriggeredSeconds :type Float%20%28double-precision%29) (InputAction :type Input%20Action%20Object%20Reference :default "/Game/FMP/Camera/Input/EnhancedInput/IA_Zoom.IA_Zoom"))
  ;[1 0.549 0.8392] Camera Zoom
  (Camera|CameraZoom ActionValue)
  (Camera|CameraSpeed))

(event Input|EnhancedActionEvents|EnhancedInputActionIA_Click
  (params (ActionValue :type Float%20%28double-precision%29) (ElapsedSeconds :type Float%20%28double-precision%29) (TriggeredSeconds :type Float%20%28double-precision%29) (InputAction :type Input%20Action%20Object%20Reference :default "/Game/FMP/Camera/Input/EnhancedInput/IA_Click.IA_Click"))
  (bind _spawned_actor (Variables|Default|GetSpawned%20actor))
  ;[0.2431 0.298 1] Place Building
  (:Started
    (Utilities|IsValid _spawned_actor
      (:Is%20Valid
        (Class|BPInterface|Remove(Message) _spawned_actor)
        (if (and (Variables|Default|GetHas%20Money) (Variables|Default|GetPlace%20Building))
          (CallFunction|PlaceBuilding)
          (Default|ChangeMoney (Variables|Default|GetWidgetREf))
          (else
            (Actor|DestroyActor (Variables|Default|GetSpawned%20actor))
            (Variables|Default|SetFollowMouse false)))))))

(event Input|EnhancedActionEvents|EnhancedInputActionIA_Turn
  (params (ActionValue :type Float%20%28double-precision%29) (ElapsedSeconds :type Float%20%28double-precision%29) (TriggeredSeconds :type Float%20%28double-precision%29) (InputAction :type Input%20Action%20Object%20Reference :default "/Game/FMP/Camera/Input/EnhancedInput/IA_Turn.IA_Turn"))
  ;[1 0.549 0.8392] Camera Rotation and Pitch
  (Camera|CamRotation ActionValue))

(event Input|EnhancedActionEvents|EnhancedInputActionIA_Pitch
  (params (ActionValue :type Float%20%28double-precision%29) (ElapsedSeconds :type Float%20%28double-precision%29) (TriggeredSeconds :type Float%20%28double-precision%29) (InputAction :type Input%20Action%20Object%20Reference :default "/Game/FMP/Camera/Input/EnhancedInput/IA_Pitch.IA_Pitch"))
  ;[1 0.549 0.8392] Camera Rotation and Pitch
  (Camera|CameraPitch ActionValue))

(event EventBeginPlay
  (bind _self self)
  (bind _asmain_game_instance (Utilities|Casting|CastToMainGameInstance (Game|GetGameInstance)))
  (Variables|Default|SetAs%20Main%20Game%20Instance _asmain_game_instance)
  (bind _asbp_camera_actor (Utilities|Casting|CastToBP_CameraActor (Game|GetPlayerCharacter 0)))
  (Variables|Default|SetAs%20BP%20Camera%20Actor _asbp_camera_actor)
  (Input|AddMappingContext (PlayerController|LocalPlayerSubsystems|GetEnhancedInputLocalPlayerSubsystem _self) "/Game/FMP/Camera/Input/CameraMovement.CameraMovement" 1 "(bIgnoreAllPressedKeysUntilRelease=True,bForceImmediately=False,bNotifyUserSettings=False)")
  (bind _returnvalue (UserInterface|CreateWidget "/Game/FMP/Camera/UI/InGame/Layouts/UI_InGame.UI_InGame_C" _self))
  (Variables|Default|SetWidgetREf _returnvalue)
  (UserInterface|Viewport|AddtoViewport _returnvalue 0)
  (Variables|Camera|SetInitial%20walk%20speed (Variables|/Script/Engine.CharacterMovementComponent|GetMaxWalkSpeed (Variables|/Script/Engine.Character|GetCharacterMovement (Variables|Default|GetAs%20BP%20Camera%20Actor))))
  (Camera|CameraSpeed)
  (Variables|Default|SetFollowMouse false))

(event EventTick
  (params (DeltaSeconds :type Float%20%28single-precision%29))
  (bind (_worldlocation _worlddirection) (Game|Player|ConvertMouseLocationToWorldSpace))
  ;[1 0.02841 0] REFACTOR THE SHIT OUT OF THIS!!!!! Makes the building follow the mouse position
  (if (Variables|Default|GetFollowMouse)
    (bind _outhit (Collision|LineTraceByChannel _worldlocation (+ _worldlocation (* _worlddirection 5e+04)) "TraceTypeQuery1" false 0 "Persistent"))
    (Transformation|SetActorLocation (Variables|Default|GetSpawned%20actor) (.Location (Collision|BreakHitResult _outhit)) false false)))

(event EventBuild
  (params (Selection :type E_Buildings%20Enum :default "NewEnumerator0") (Cost :type Integer))
  ;[0.2431 0.298 1] Change Building Type
  (if (> Cost (Variables|/Game/FMP/Camera/MainGameInstance.MainGameInstance_C|GetMoney (Variables|Default|GetAs%20Main%20Game%20Instance)))
    (Utilities|IsValid (Variables|Default|GetSpawned%20actor)
      (:Is%20Valid
        (Actor|DestroyActor (Variables|Default|GetSpawned%20actor))
        (Variables|Default|SetPlace%20Building false)
        (Variables|Default|SetFollowMouse false)))
    (else
      (CallFunction|BuildingType Selection)
      (CallFunction|CanFollowMouse)
      (Variables|Default|SetHas%20Money true)
      (Variables|Default|SetPlace%20Building true))))

(event EventRemove
  (Class|BPIUI|StopAnim(Message) (Variables|Default|GetWidgetREf)))

(fn ConstructionScript)

(fn MoveCamera)

(fn PlaceBuilding
  (bind (_worldlocation _worlddirection) (Game|Player|ConvertMouseLocationToWorldSpace))
  (bind _outhit (Collision|LineTraceByChannel _worldlocation (+ _worldlocation (* _worlddirection 5e+04)) "TraceTypeQuery1" false 0 "Persistent"))
  (if (.bBlockingHit (Collision|BreakHitResult _outhit))
    (bind _returnvalue (Game|SpawnActorfromClass (Variables|Default|GetBuilding%20Class) (Math|Transform|MakeTransform (.Location (Collision|BreakHitResult _outhit)) "0, 0, 0" "1.000000,1.000000,1.000000") "Undefined" "MultiplyWithRoot" (.HitActor (Collision|BreakHitResult _outhit)) 0))
    (Class|BPInterface|Interact(Message) _returnvalue)))

(fn CameraZoom
  (params (A :type Float%20%28double-precision%29))
  (bind _as_bp_camera_actor (Variables|Default|GetAs%20BP%20Camera%20Actor))
  (bind _springarm (Variables|/Game/FMP/Camera/BP_CameraActor.BP_CameraActor_C|GetSpringArm _as_bp_camera_actor))
  (Variables|/Script/Engine.SpringArmComponent|SetTargetArmLength _springarm (Math|Float|Clamp(Float) (+ (Variables|/Script/Engine.SpringArmComponent|GetTargetArmLength _springarm) (* A 5e+01)) (Variables|Camera|GetMin%20Arm%20Length) (Variables|Camera|GetMax%20Arm%20Length))))

(fn Moving
  (params (B :type Float%20%28double-precision%29) (B2 :type Float%20%28double-precision%29))
  (bind _self self)
  (Pawn|Input|AddMovementInput (Variables|Default|GetAs%20BP%20Camera%20Actor) (+ (* (Transformation|GetActorRightVector _self) B) (* (Transformation|GetActorForwardVector _self) B2)) 1.0 false))

(fn CameraSpeed
  (bind _as_bp_camera_actor (Variables|Default|GetAs%20BP%20Camera%20Actor))
  (Variables|/Script/Engine.CharacterMovementComponent|SetMaxWalkSpeed (Variables|/Script/Engine.Character|GetCharacterMovement _as_bp_camera_actor) (* (Variables|Camera|GetInitial%20walk%20speed) (/ (Variables|/Script/Engine.SpringArmComponent|GetTargetArmLength (Variables|/Game/FMP/Camera/BP_CameraActor.BP_CameraActor_C|GetSpringArm _as_bp_camera_actor)) (Variables|Camera|GetMin%20Arm%20Length)))))

(fn CameraPitch
  (params (A :type Float%20%28double-precision%29))
  (bind _as_bp_camera_actor (Variables|Default|GetAs%20BP%20Camera%20Actor))
  (bind _springarm (Variables|/Game/FMP/Camera/BP_CameraActor.BP_CameraActor_C|GetSpringArm _as_bp_camera_actor))
  (bind _returnvalue (Transformation|GetWorldRotation _springarm))
  (Transformation|SetWorldRotation _springarm (Math|Rotator|MakeRotator (.roll _returnvalue) (Math|Float|ClampAngle (+ (* A 0.5) (.pitch _returnvalue)) (Variables|Camera|Getcam%20Min%20clamp) (Variables|Camera|Getcam%20max%20clamp)) (.yaw _returnvalue)) false false))

(fn CamRotation
  (params (A :type Float%20%28double-precision%29))
  (Pawn|Input|AddControllerYawInput (Variables|Default|GetAs%20BP%20Camera%20Actor) (* A 0.5)))

(fn BuildingType
  (params (Selection :type E_Buildings%20Enum :default "NewEnumerator0"))
  (switch Utilities|FlowControl|Switch|SwitchonE_Buildings Selection
    (:NewEnumerator0
      (Variables|Default|SetBuilding%20Class "/Game/FMP/Buildings/Housing/BP_Tent.BP_Tent_C"))
    (:NewEnumerator1
      (Variables|Default|SetBuilding%20Class "/Game/FMP/Buildings/Housing/BP_Shack.BP_Shack_C"))
    (:NewEnumerator2
      (Variables|Default|SetBuilding%20Class "/Game/FMP/Buildings/Housing/BP_House.BP_House_C"))
    (:NewEnumerator3
      (Variables|Default|SetBuilding%20Class "/Game/FMP/Buildings/Nautical/BP_Dock.BP_Dock_C"))
    (:NewEnumerator4
      (Variables|Default|SetBuilding%20Class "/Game/FMP/Buildings/Nautical/BP_ShipYard.BP_ShipYard_C"))
    (:NewEnumerator5
      (Variables|Default|SetBuilding%20Class "/Game/FMP/Buildings/Nautical/BP_Cartography.BP_Cartography_C"))
    (:NewEnumerator6
      (Variables|Default|SetBuilding%20Class "/Game/FMP/Buildings/Produciton/BP_GunSmith.BP_GunSmith_C"))
    (:NewEnumerator7
      (Variables|Default|SetBuilding%20Class "/Game/FMP/Buildings/Produciton/BP_BlackSmith.BP_BlackSmith_C"))
    (:NewEnumerator8
      (Variables|Default|SetBuilding%20Class "/Game/FMP/Buildings/Produciton/BP_RumDistillery.BP_RumDistillery_C")))
  (bind _returnvalue (Game|SpawnActorfromClass (Variables|Default|GetBuilding%20Class) (Math|Transform|MakeTransform "0, 0, 0" "0, 0, 0" "1.000000,1.000000,1.000000") "Undefined" "MultiplyWithRoot" 0 0))
  (Variables|Default|SetSpawned%20actor _returnvalue))